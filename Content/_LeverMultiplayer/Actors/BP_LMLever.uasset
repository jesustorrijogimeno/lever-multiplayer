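; BP_LMLever is a lever actor for the LeverMultiplayer content that shows and hides its on-screen info widget.
; The ShowUI event calls ShowUIInfo, which creates a BP_LMLeverWidget, stores it in Info and adds it to the viewport only if none exists.
; DisableUI calls DisableUIInfo, which removes that widget and clears the reference so it can be recreated.
; The file contains no lever interaction or replication logic.
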(event EventShowUI
  (CallFunction|ShowUIInfo))

(event EventDisableUI
  (CallFunction|DisableUIInfo))

(fn ConstructionScript)

(fn ShowUIInfo
  (if (not (Utilities|IsValid (Variables|Default|GetInfo)))
    (bind _returnvalue (UserInterface|CreateWidget "/Game/_LeverMultiplayer/UI/Lever/BP_LMLeverWidget.BP_LMLeverWidget_C" 0 self))
    (Variables|Default|SetInfo _returnvalue)
    (UserInterface|Viewport|AddtoViewport _returnvalue 0)))

(fn DisableUIInfo
  (if (Utilities|IsValid (Variables|Default|GetInfo))
    (Widget|RemovefromParent (Variables|Default|GetInfo))
    (Variables|Default|SetInfo 0)))